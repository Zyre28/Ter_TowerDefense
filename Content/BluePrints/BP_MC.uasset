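; BP_MC is the player-controlled character, which moves around and places plants on a grid.
; Forward and right inputs add movement relative to the control rotation's yaw.
; Pressing E or Space looks up the GridManager, converts the character's location to a row and column, and asks it to spawn BP_PlantBullet there.
; Failed conversions and key releases only print debug strings.
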(event `self.ReceiveBeginPlay`
  (`GameplayStatics.GetActorOfClass` "/Script/TER_TowerDefense.GridManager"))

(event `Key|E`
  (params (Key :type "Key Structure"))
  (:`Pressed`
    (bind _returnvalue (`GameplayStatics.GetActorOfClass` "/Script/TER_TowerDefense.GridManager" :!label _label))
    (bind (_outrow _outcol _returnvalue_2) (`GridManager.WorldToGrid` _returnvalue (`self.K2_GetActorLocation`)))
    (if _returnvalue_2
      (`GridManager.SpawnPlant` _returnvalue "/Game/BluePrints/BP_PlantBullet.BP_PlantBullet_C" _outrow _outcol)
      (else
        (`KismetSystemLibrary.PrintString` "DEAD"))))
  (:`Released`
    (`KismetSystemLibrary.PrintString` "RELEASED" :!label _label_2)))

(event `Key|SpaceBar`
  (params (Key :type "Key Structure"))
  (:`Pressed`
    (goto _label))
  (:`Released`
    (goto _label_2)))

(event `EnhancedInput|/Game/Inputs/Move_Forward`
  (params (ActionValue :type "Float (double-precision)") (ElapsedSeconds :type "Float (double-precision)") (TriggeredSeconds :type "Float (double-precision)") (InputAction :type "InputAction Object Reference" :default "/Game/Inputs/Move_Forward.Move_Forward"))
  (bind (_returnvalue_roll _returnvalue_pitch _returnvalue_yaw) (`KismetMathLibrary.BreakRotator` (`self.GetControlRotation`)))
  (:`Triggered`
    (`self.AddMovementInput` (`KismetMathLibrary.GetForwardVector` (`KismetMathLibrary.MakeRotator` 0.0 0.0 _returnvalue_yaw)) ActionValue)))

(event `EnhancedInput|/Game/Inputs/Move_Right`
  (params (ActionValue :type "Float (double-precision)") (ElapsedSeconds :type "Float (double-precision)") (TriggeredSeconds :type "Float (double-precision)") (InputAction :type "InputAction Object Reference" :default "/Game/Inputs/Move_Right.Move_Right"))
  (bind (_returnvalue_roll _returnvalue_pitch _returnvalue_yaw) (`KismetMathLibrary.BreakRotator` (`self.GetControlRotation`)))
  (:`Triggered`
    (`self.AddMovementInput` (`KismetMathLibrary.GetRightVector` (`KismetMathLibrary.MakeRotator` 0.0 0.0 _returnvalue_yaw)) ActionValue)))

(fn `UserConstructionScript`)